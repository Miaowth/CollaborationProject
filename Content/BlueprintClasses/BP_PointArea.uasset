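; Scoring zone tied to one player that totals the point value of trash inside its box and adjusts that player's speed.
; Each trash overlap begin or end triggers a fresh box-overlap recount and prints the total.
; Component tags mark buff and debuff trash, whose counts and last-read amounts set the net value passed to AlterSpeed.
; Trash on a boundary between areas counts toward both totals.
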(event OnComponentBeginOverlap(Box)
  (params (OverlappedComponent :type Primitive%20Component%20Object%20Reference) (OtherActor :type Actor%20Object%20Reference) (OtherComp :type Primitive%20Component%20Object%20Reference) (OtherBodyIndex :type Integer) (bFromSweep :type Boolean) (SweepResult :type Hit%20Result%20Structure%20%28by%20ref%29))
  (Utilities|Casting|CastToBP_MasterTrash OtherActor)
  (CallFunction|CalculatePointTotal)
  (Development|PrintString (Utilities|String|Append "Player " (Utilities|String|ToString(Integer) (Variables|Default|GetPlayerNumber)) ": " (Utilities|String|ToString(Integer) (Variables|Default|GetTotalPoints)))))

(event Custom|CalculateBuffs
  (Default|AlterSpeed (Variables|Default|GetPlayerRef) (+ (* (Variables|Default|GetTrashBuffNum) (Variables|Default|GetPlayerBuffAmount)) (* (* (Variables|Default|GetTrashDebuffNum) (Variables|Default|GetPlayerDebuffAmount)) -1.0))))

(event EventBeginPlay
  (bind _playerref (Variables|Default|GetPlayerRef))
  ;[0.257 1 0.2402] Begin Play
  (Variables|Default|SetPlayerNumber (Variables|/Game/BlueprintClasses/BP_Character.BP_Character_C|GetPlayerID _playerref))
  (Variables|Default|SetDefaultMoveSpeed (Variables|/Script/Engine.CharacterMovementComponent|GetMaxWalkSpeed (Variables|/Script/Engine.Character|GetCharacterMovement _playerref))))

(event Collision|EventActorEndOverlap
  (params (OtherActor :type Actor%20Object%20Reference))
  (Utilities|Casting|CastToBP_MasterTrash OtherActor)
  (CallFunction|CalculatePointTotal)
  (Development|PrintString (Utilities|String|Append "Player " (Utilities|String|ToString(Integer) (Variables|Default|GetPlayerNumber)) ": " (Utilities|String|ToString(Integer) (Variables|Default|GetTotalPoints)))))

(fn ConstructionScript)

(fn CalculatePointTotal
  (bind _box (Variables|Default|GetBox))
  ;[1 0.4077 0.7458] adds together the points for each item that overlaps with the area. If trash is on a boundary, then it counts towards both totals
  (Variables|Default|SetTotalBuffs 0)
  (Variables|Default|SetTrashBuffNum 0)
  (Variables|Default|SetTrashDebuffNum 0)
  (Variables|Default|SetCurrentPoints 0)
  (bind _outactors (Collision|BoxOverlapActors (Transformation|GetWorldLocation _box) (Components|Box|GetScaledBoxExtent _box) (Utilities|Array|MakeArray "ObjectTypeQuery8") "/Game/BlueprintClasses/BP_MasterTrash.BP_MasterTrash_C" :!class /Script/Engine.KismetSystemLibrary))
  (for _array_element _outactors
    (bind _asbp_master_trash (Utilities|Casting|CastToBP_MasterTrash _array_element))
    (if (or (Components|ComponentHasTag (Variables|/Game/BlueprintClasses/BP_MasterTrash.BP_MasterTrash_C|GetStaticMesh _asbp_master_trash) "TrashBuff") (Components|ComponentHasTag (Variables|/Game/BlueprintClasses/BP_MasterTrash.BP_MasterTrash_C|GetStaticMesh _asbp_master_trash) "TrashDebuff"))
      (if (Components|ComponentHasTag (Variables|/Game/BlueprintClasses/BP_MasterTrash.BP_MasterTrash_C|GetStaticMesh _asbp_master_trash) "TrashBuff")
        (bind _result (Math|Integer|IncrementInt (Variables|Default|GetTrashBuffNum))
          (:%20%20
            (Variables|Default|SetTrashBuffNum _result)
            (Variables|Default|SetPlayerBuffAmount (Variables|/Game/BlueprintClasses/BP_MasterTrash.BP_MasterTrash_C|GetBuffAmount _asbp_master_trash))))
        (else
          (bind _result_2 (Math|Integer|IncrementInt (Variables|Default|GetTrashDebuffNum))
            (:%20%20
              (Variables|Default|SetTrashDebuffNum _result_2)
              (Variables|Default|SetPlayerDebuffAmount (Variables|/Game/BlueprintClasses/BP_MasterTrash.BP_MasterTrash_C|GetBuffAmount _asbp_master_trash)))))))
    (Variables|Default|SetCurrentPoints (+ (Variables|/Game/BlueprintClasses/BP_MasterTrash.BP_MasterTrash_C|GetPointValue _asbp_master_trash) (Variables|Default|GetCurrentPoints))))
  (if (== (Variables|Default|GetTrashBuffNum) 0)
    (Variables|Default|SetPlayerBuffAmount 0.0))
  (if (== (Variables|Default|GetTrashDebuffNum) 0)
    (Variables|Default|SetPlayerDebuffAmount 0.0))
  (CallFunction|CalculateBuffs)
  (bind _output_get (Variables|Default|SetTotalPoints (Variables|Default|GetCurrentPoints)))
  (return _output_get))
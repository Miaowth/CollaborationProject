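; Hub-world level gate that loads the level named by LevelName once the number of overlapping BP_Characters equals NumOfPlayers.
; On that overlap it appends each character's ID and colour to PlayerInfo in BP_GameInstance, then opens the level after a short delay.
; Leaving the gate does nothing, as the player-removal logic is disconnected, so a started load is not cancelled.
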(event EventBeginPlay
  (Variables|Default|SetGameinstRef (.AsBP%20Game%20Instance (Utilities|Casting|CastToBP_GameInstance (Game|GetGameInstance)))))

(event Collision|EventActorBeginOverlap
  (params (OtherActor :type Actor%20Object%20Reference))
  (bind _overlappingactors (Collision|GetOverlappingActors "/Game/BlueprintClasses/BP_Character.BP_Character_C" :!class /Script/Engine.Actor))
  (if (== (Utilities|Array|Length _overlappingactors) (Variables|Default|GetNumOfPlayers))
    (for _array_element _overlappingactors
      (bind _asbp_character (Utilities|Casting|CastToBP_Character _array_element))
      (bind _returnvalue (Utilities|Array|Add (Variables|/Game/BlueprintClasses/HubWorld/BP_GameInstance.BP_GameInstance_C|GetPlayerInfo (Variables|Default|GetGameinstRef)) (Utilities|Struct|MakeStruct_PlayerData (Variables|/Game/BlueprintClasses/BP_Character.BP_Character_C|GetPlayerID _asbp_character) (Variables|/Game/BlueprintClasses/BP_Character.BP_Character_C|GetPlayerColour _asbp_character))))
      (Development|PrintString (Utilities|String|ToString(Integer) _returnvalue)))
    (Utilities|FlowControl|Delay 2.0)
    (Game|OpenLevel(byName) (Variables|Default|GetLevelName))))

(event Collision|EventActorEndOverlap
  (params (OtherActor :type Actor%20Object%20Reference)))

(fn ConstructionScript)
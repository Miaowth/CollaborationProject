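; Player character that runs, jumps, picks up BP_MasterTrash objects and throws them, with a brief input-disabling stun.
; A sphere trace grabs unheld trash into a PhysicsHandle that follows TrashPoint and the Cube, which interpolates toward the input direction.
; Holding Throw opens a Tick-driven gate that charges power and drives the WBP_PowerBar widget; release launches the trash along ThrowAim.
; A looping timer and jump/land events toggle running particles.
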(event Custom|DropTrash
  (bind _powerbarref (Variables|Default|GetPowerBarRef))
  ;[1 0.6805 0.0317] PickUp + Throw
  (Utilities|IsValid (Variables|Default|GetTrashHeld)
    (:Is%20Valid
      (Physics|Components|PhysicsHandle|ReleaseComponent (Variables|Default|GetPhysicsHandle))
      (Physics|AddImpulse (stale Input|ActionEvents|InputActionPickup _output_get) (* (Math|Vector|GetForwardVector (Variables|Default|GetThrowAim)) (* (Variables|Default|GetPowerAmount) (Variables|Default|GetPowerMult))) "None" true)
      (Collision|SetCollisionResponsetoChannel (stale Input|ActionEvents|InputActionPickup _output_get) "ECC_GameTraceChannel1" "ECR_Block")
      (Collision|SetCollisionResponsetoChannel (stale Input|ActionEvents|InputActionPickup _output_get) "ECC_GameTraceChannel2" "ECR_Block")
      (Variables|/Game/BlueprintClasses/BP_MasterTrash.BP_MasterTrash_C|SetHeld? (Variables|Default|GetTrashOwner) false)
      (Variables|Default|SetTrashOwner 0)
      (Variables|Default|SetTrashHeld 0)
      (Variables|Default|SetPowerMult 0.0)
      (Class|UserWidget|StopAnimation _powerbarref (Variables|/Game/BlueprintClasses/Widgets/WBP_PowerBar.WBP_PowerBar_C|GetMaxPower _powerbarref))
      (Default|ResetTransform _powerbarref)
      (CallFunction|ResetMaxPower)
      (Variables|Default|SetHolding? false))))

(event Custom|ThrowCharge
  ;[1 0.6805 0.0317] PickUp + Throw
  (Utilities|FlowControl|Gate true
    (:Exit
      (bind _output_get (Variables|Default|SetPowerMult (Math|Float|Clamp(Float) (+ (Variables|Default|GetPowerMult) (Utilities|Time|GetWorldDeltaSeconds)) 0.0 (Variables|Default|GetMaxPower))))
      (if (== _output_get (Variables|Default|GetMaxPower))
        (Utilities|FlowControl|DoOnce false
          (:Completed
            (Default|PowerMax (Variables|Default|GetPowerBarRef))))))))

(event Custom|ResetMaxPower
  ;[1 0.6805 0.0317] PickUp + Throw
  (Utilities|FlowControl|DoOnce false) ; enters at Reset
)

(event Custom|CheckMovement
  (bind _ps_running (Variables|Default|GetPS_Running))
  ;[1 1 1] Particle system
  (if (and (AI|Components|NavMovement|IsMovingonGround (Variables|Character|GetCharacterMovement)) (!= (Input|AxisValues|GetMove_foward) (Input|AxisValues|GetMove_Right)))
    (if (not (AI|Components|NavMovement|IsFalling (Variables|Character|GetCharacterMovement)))
      (Components|Activation|SetActive _ps_running true false))
    (else
      (Components|Activation|SetActive _ps_running false false))))

(event Custom|Stun
  (bind _returnvalue (Game|GetPlayerController 0))
  (Input|DisableInput _returnvalue)
  (Utilities|FlowControl|Delay 1.0)
  (Input|EnableInput _returnvalue))

(event EventBeginPlay
  ;[0 1 0.3688] Beginplay
  (bind _returnvalue (UserInterface|CreateWidget "/Game/BlueprintClasses/Widgets/WBP_PowerBar.WBP_PowerBar_C" 0 self))
  (bind _output_get (Variables|Default|SetPowerBarRef _returnvalue))
  (UserInterface|SetWidget (Variables|Default|GetPowerBar) _output_get)
  ;[1 1 1] Particle system
  (Utilities|Time|SetTimerbyEvent (delegate Custom|CheckMovement) 0.2 true))

(event EventOnLanded
  (params (Hit :type Hit%20Result%20Structure%20%28by%20ref%29))
  ;[0.5925 0.9701 1] Movement
  (Components|Activation|SetActive (Variables|Default|GetPS_Running) true false))

(event EventTick
  (params (DeltaSeconds :type Float%20%28single-precision%29))
  ;[1 0.08993 0.1696] Tick
  (Class|PhysicsHandleComponent|SetTargetLocationandRotation (Variables|Default|GetPhysicsHandle) (Transformation|GetWorldLocation (Variables|Default|GetTrashPoint)) (Transformation|GetWorldRotation (Variables|Default|GetCube)))
  (CallFunction|ThrowCharge))

(event Input|ActionEvents|InputActionJomp
  (params (Key :type Key%20Structure :default "None"))
  ;[0.5925 0.9701 1] Movement
  (:Pressed
    (Character|Jump)
    (Components|Activation|SetActive (Variables|Default|GetPS_Running) false false)))

(event Input|ActionEvents|InputActionPickup
  (params (Key :type Key%20Structure :default "None"))
  (bind _pickupaim (Variables|Default|GetPickupAim))
  (bind _returnvalue (Transformation|GetWorldLocation _pickupaim))
  ;[1 0.6805 0.0317] PickUp + Throw
  (:Pressed
    (if (not (Variables|Default|GetHolding?))
      (bind (_outhit _returnvalue_2) (Collision|SphereTraceForObjects _returnvalue (+ _returnvalue (* (Math|Vector|GetForwardVector _pickupaim) 75.0)) 75.0 (Utilities|Array|MakeArray "ObjectTypeQuery8") false 0 "ForOneFrame" true "(R=1.000000,G=0.000000,B=0.000000,A=1.000000)" "(R=0.000000,G=1.000000,B=0.000000,A=1.000000)" 1.0))
      (if _returnvalue_2
        (bind _asbp_master_trash (Utilities|Casting|CastToBP_MasterTrash (Components|GetOwner (.HitComponent (Collision|BreakHitResult _outhit)))))
        (if (not (Variables|/Game/BlueprintClasses/BP_MasterTrash.BP_MasterTrash_C|GetHeld? _asbp_master_trash))
          (Variables|/Game/BlueprintClasses/BP_MasterTrash.BP_MasterTrash_C|SetHeld? _asbp_master_trash true)
          (Variables|Default|SetHolding? true)
          (Variables|Default|SetTrashOwner _asbp_master_trash)
          (bind _output_get (Variables|Default|SetTrashHeld (.HitComponent (Collision|BreakHitResult _outhit))))
          (Collision|SetCollisionResponsetoChannel _output_get "ECC_GameTraceChannel1" "ECR_Ignore")
          (Collision|SetCollisionResponsetoChannel _output_get "ECC_GameTraceChannel2" "ECR_Ignore")
          (Physics|Components|PhysicsHandle|GrabComponentatLocationwithRotation (Variables|Default|GetPhysicsHandle) _output_get "None" (Transformation|GetWorldLocation _output_get) (Transformation|GetWorldRotation (Variables|Default|GetCube))))))))

(event Input|ActionEvents|InputActionThrow
  (params (Key :type Key%20Structure :default "None"))
  (bind _holding_ (Variables|Default|GetHolding?))
  (bind _powerbarref (Variables|Default|GetPowerBarRef))
  ;[1 0.6805 0.0317] PickUp + Throw
  (:Pressed
    (if _holding_
      (Default|ShowBar _powerbarref)
      (Utilities|FlowControl|Gate true) ; enters at Open
    ))
  (:Released
    (if _holding_
      (Default|HideBar _powerbarref)
      (Utilities|FlowControl|Delay 0.1)
      (CallFunction|DropTrash)
      (Utilities|FlowControl|Gate true) ; enters at Close
    )))

(event Input|AxisEvents|InputAxisMove_Right
  (params (AxisValue :type Float%20%28single-precision%29))
  ;[0.5925 0.9701 1] Movement
  (Pawn|Input|AddMovementInput (Transformation|GetActorRightVector) AxisValue false))

(event Input|AxisEvents|InputAxisMove_foward
  (params (AxisValue :type Float%20%28single-precision%29))
  (bind _returnvalue (Input|AxisValues|GetMove_foward))
  (bind _returnvalue_2 (Input|AxisValues|GetMove_Right))
  (bind _cube (Variables|Default|GetCube))
  ;[0.5925 0.9701 1] Movement
  (Pawn|Input|AddMovementInput (Transformation|GetActorForwardVector) AxisValue false)
  (Transformation|SetRelativeRotation _cube (Math|Interpolation|RInterpTo (Variables|/Script/Engine.SceneComponent|GetRelativeRotation _cube) (Variables|Default|GetLookingDir) (Utilities|Time|GetWorldDeltaSeconds) 7.5) false false)
  (if (or (!= _returnvalue 0.0) (!= _returnvalue_2 0.0))
    (Variables|Default|SetLookingDir (Math|Rotator|MakeRotfromX (Math|Vector|MakeVector _returnvalue _returnvalue_2 0.0)))))

(fn ConstructionScript)
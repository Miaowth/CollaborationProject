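; BP_SharkSpawner is a spawner actor that periodically launches sharks from its own transform.
; A looping timer set on BeginPlay spawns a BP_Shark every ten seconds.
; Each new shark's skeletal mesh receives a velocity-change impulse, strong along the spawner's local up axis with random sideways spread, so the actor's rotation aims the launch.
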(event Custom|SpawnShark
  (bind _returnvalue (Game|SpawnActorfromClass "/Game/BlueprintClasses/BP_Shark.BP_Shark_C" (Transformation|GetActorTransform) "Undefined" 0 0))
  (Physics|AddImpulse (Variables|/Game/BlueprintClasses/BP_Shark.BP_Shark_C|GetSkeletalMesh _returnvalue) (Math|Vector|RotateVector (Math|Vector|MakeVector (Math|Random|RandomFloatinRange -2.5e+02 2.5e+02) (Math|Random|RandomFloatinRange -2.5e+02 2.5e+02) (Math|Random|RandomFloatinRange 2.5e+03 2.5e+03)) (Transformation|GetActorRotation)) "None" true))

(event EventBeginPlay
  (Utilities|Time|SetTimerbyEvent (delegate Custom|SpawnShark) 1e+01 true))

(fn ConstructionScript)
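; Trash spawner actor that registers with BP_GM and launches BP_MasterTrash actors from its own transform.
; StartSpawn runs a looping timer, paused by StopSpawning, that triggers either a single spawn or, by weighted chance, a random-sized burst.
; The TrashSpawn macro staggers bursts with a DoN and Delay loop, looks up a random BP_TrashTable row, applies a random upward impulse, then resets.
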(event Custom|SpawnTrash
  (if (Math|Random|RandomBoolwithWeight (Variables|Default|GetMoretrashChance))
    (bind _output_get (Variables|Default|SetTrashToSpawn (Math|Random|RandomIntegerinRange (Variables|Default|GetTrashMin) (Variables|Default|GetTrashMax))))
    (Utilities|TrashSpawn _output_get)
    (else
      (bind _output_get_2 (Variables|Default|SetTrashToSpawn 1))
      (Utilities|TrashSpawn _output_get_2))))

(event Custom|ResetSpawn
  (Utilities|FlowControl|Sequence
    (:then_0
      (Utilities|TrashSpawn (stale Custom|SpawnTrash _output_get)) ; enters at Reset
    )
    (:then_1
      (Utilities|TrashSpawn (stale Custom|SpawnTrash _output_get_2)) ; enters at Reset
    )))

(event Custom|StopSpawning
  (Utilities|Time|PauseTimerbyHandle (stale Custom|StartSpawn _returnvalue)))

(event Custom|StartSpawn
  (bind _returnvalue (Utilities|Time|SetTimerbyEvent (delegate Custom|SpawnTrash) 3.0 true 1.0 2.0)))

(event EventBeginPlay
  (bind _asbp_gm (Utilities|Casting|CastToBP_GM (Game|GetGameMode)))
  (Variables|/Game/BlueprintClasses/BP_GM.BP_GM_C|SetSpawnerRef _asbp_gm self))

(fn ConstructionScript)
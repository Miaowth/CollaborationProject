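; Game mode for a timed local multiplayer minigame where players score through point areas.
; BeginPlay spawns and possesses a coloured character per GameInstance player, shuffles them across point areas, and shows the title screen over a shared camera.
; StartGame starts music, timer UI, spawner and score displays, while Tick runs the clock and final-seconds countdown sound.
; At zero, it picks the top-scoring area's team or a tie, shows the end screen and returns to Hub_World.
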(event Custom|PlayEnvironment
  (Audio|PlaySound2D "/Game/Assets/Audio/SoundFX/Environment/GeneralEnvironment.GeneralEnvironment" 1.0 1.0 0.0 0 0))

(event Custom|StartGame
  (Audio|Components|Audio|Play (Variables|Default|Getbg_music) 0.0)
  (Default|Remove (stale EventBeginPlay _returnvalue_2))
  (Utilities|FlowControl|Delay 2.5)
  (bind _returnvalue (UserInterface|CreateWidget "/Game/BlueprintClasses/Widgets/WBP_Timer.WBP_Timer_C" 0 self))
  (bind _output_get (Variables|Default|SetTimerRef _returnvalue))
  (UserInterface|Viewport|AddtoViewport _output_get 0)
  (Default|StartSpawn (Variables|Default|GetSpawnerRef))
  (for _array_element (Variables|Default|GetPointAreaRefs)
    (Default|ShowScore _array_element))
  (Variables|Default|SetIsTimerActive true))

(event Custom|PlayCountdown
  (Audio|PlaySound2D "/Game/Assets/Audio/SoundFX/TimerEffect2.TimerEffect2" 1.0 1.0 0.0 0 0))

(event EventBeginPlay
  (bind _activeplayers (Variables|Default|GetActivePlayers))
  (bind _pointarearefs (Variables|Default|GetPointAreaRefs))
  (bind _pointareaindex (Variables|Default|GetPointAreaIndex))
  (for _index (range 0 3)
    _)
  (bind _output_get (Variables|Default|SetGameInstRef (.AsBP%20Game%20Instance (Utilities|Casting|CastToBP_GameInstance (Game|GetGameInstance)))))
  (for (_array_element _array_index) (Variables|/Game/BlueprintClasses/HubWorld/BP_GameInstance.BP_GameInstance_C|GetPlayerInfo _output_get)
    (bind _returnvalue (Game|SpawnActorfromClass "/Game/BlueprintClasses/BP_Character.BP_Character_C" (Math|Transform|MakeTransform (Math|Vector|MakeVector (Math|Random|RandomFloatinRange -5e+02 5e+02) (Math|Random|RandomFloatinRange -5e+02 5e+02) 2e+02) "0,90.000000, 0" "1,1,1") "Undefined" 0 0)) ; Z Rotation set to 90 so they face the right way
    (Variables|/Game/BlueprintClasses/BP_Character.BP_Character_C|SetPlayerID _returnvalue (.PlayerID (Utilities|Struct|BreakStruct_PlayerData _array_element)))
    (Variables|/Game/BlueprintClasses/BP_Character.BP_Character_C|SetPlayerColour _returnvalue (.PlayerCol (Utilities|Struct|BreakStruct_PlayerData _array_element)))
    (Default|UpdateColour _returnvalue)
    (Pawn|Possess (Game|GetPlayerController _array_index) _returnvalue)
    (Utilities|Array|Add (Variables|/Game/BlueprintClasses/BP_WorldCamera.BP_WorldCamera_C|GetPlayerRefArray (Variables|Default|GetCameraRef)) _returnvalue)
    (Utilities|Array|Add (Variables|Default|GetActivePlayers) _returnvalue))
  (Utilities|Array|Shuffle _activeplayers)
  (for _array_element_2 _activeplayers
    (Utilities|Array|Add (Variables|/Game/BlueprintClasses/BP_PointArea.BP_PointArea_C|GetTeamRefs (Utilities|Array|Get(acopy) _pointarearefs (Variables|Default|GetPointAreaIndex))) _array_element_2)
    (if (< _pointareaindex (- (Utilities|Array|Length _pointarearefs) 1))
      (Math|Integer|IncrementInt _pointareaindex)))
  (Utilities|Time|SetTimerbyEvent (delegate Custom|PlayEnvironment) 1e+01 false 5.0 5.0)
  (Game|Player|SetViewTargetwithBlend (Game|GetPlayerController 0) (Variables|Default|GetCameraRef) 0.0 "VTBlend_Linear" 0.0 false)
  (bind _returnvalue_2 (UserInterface|CreateWidget "/Game/BlueprintClasses/Widgets/WBP_TitleScreen.WBP_TitleScreen_C" 0 0))
  (UserInterface|Viewport|AddtoViewport _returnvalue_2 0))

(event EventTick
  (params (DeltaSeconds :type Float%20%28single-precision%29))
  (if (Variables|Default|GetIsTimerActive)
    (bind _output_get (Variables|Default|SetCurrentTime (- (Variables|Default|GetCurrentTime) DeltaSeconds)))
    (Variables|Default|SetRealtime (Math|Float|Ceil _output_get))
    (if (<= _output_get 0.0)
      (Utilities|Time|ClearTimerbyFunctionName 0 "PlayCountdown")
      (Default|StopSpawning (Variables|Default|GetSpawnerRef))
      (Variables|Default|SetIsLastFiveSeconds false)
      (Variables|Default|SetIsTimerActive false)
      ;[1 0.4689 0.8391] checks if there is a winner or a tie
      (bind _winningplayernum (CallFunction|FindWinningPlayer))
      (if (!= _winningplayernum -1)
        (Variables|Default|SetWinnerPlayer _winningplayernum)
        (else
          (Variables|Default|SetWinnerPlayer -1)))
      (Widget|RemovefromParent (Variables|Default|GetTimerRef))
      (bind _returnvalue (UserInterface|CreateWidget "/Game/BlueprintClasses/Widgets/WBP_EndScreen.WBP_EndScreen_C" 0 self))
      (UserInterface|Viewport|AddtoViewport _returnvalue 0)
      (Utilities|FlowControl|Delay 5.5)
      (Audio|Components|Audio|Stop (Variables|Default|Getbg_music))
      (Game|OpenLevel(byName) "Hub_World")
      (elif (and (<= _output_get 5.0) (not (Variables|Default|GetIsLastFiveSeconds)))
        (Variables|Default|SetIsLastFiveSeconds true)
        (Utilities|Time|SetTimerbyEvent (delegate Custom|PlayCountdown) 1.0 true)))))

(fn ConstructionScript)

(fn FindWinningPlayer
  (for (_array_element _array_index) (Variables|Default|GetPointAreaRefs)
    (bind _pointtotal (Default|CalculatePointTotal _array_element))
    (if (> _pointtotal (LocalVariables|GetTopScore))
      (LocalVariables|SetTopScoreIndex _array_index)
      (LocalVariables|SetTopScore _pointtotal)
      (LocalVariables|SetCurrentTopPlayer (Variables|/Game/BlueprintClasses/BP_PointArea.BP_PointArea_C|GetTeamNumber _array_element))
      (elif (== _pointtotal (LocalVariables|GetTopScore))
        ;[1 0.4324 0.8792] sets top player back to -1 to indicate no current leader
        (LocalVariables|SetTopScoreIndex -1)
        (LocalVariables|SetCurrentTopPlayer -1))))
  (if (!= (LocalVariables|GetCurrentTopPlayer) -1)
    (LocalVariables|SetTopPlayer (LocalVariables|GetCurrentTopPlayer))
    (else
      (LocalVariables|SetTopPlayer -1)))
  (return (LocalVariables|GetTopPlayer)))
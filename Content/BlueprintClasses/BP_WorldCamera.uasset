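; BP_WorldCamera is a shared camera that frames all players in PlayerRefArray, registering itself as CameraRef in BP_GM on BeginPlay.
; Each tick, TickCamera moves the pivot to an offset from the players' average location and rotates it toward that average.
; The largest pairwise player distance sets a clamped spring arm length, zooming out as players spread.
; An invalid player skips the update; debug prints and an unused two-player version remain.
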(event EventTick
  (params (DeltaSeconds :type Float%20%28single-precision%29))
  (CallFunction|TickCamera))

(event EventBeginPlay
  (bind _asbp_gm (Utilities|Casting|CastToBP_GM (Game|GetGameMode)))
  (Variables|/Game/BlueprintClasses/BP_GM.BP_GM_C|SetCameraRef _asbp_gm self))

(fn ConstructionScript)

(fn TickCamera
  (bind _array_element (Utilities|Array|ForEachLoopwithBreak (Variables|Default|GetPlayerRefArray) :!label _label)
    (:LoopBody
      (if (Utilities|IsValid _array_element)
        (LocalVariables|SetTotalPlayerLocationVectors (+ (Transformation|GetActorLocation _array_element) (LocalVariables|GetTotalPlayerLocationVectors)))
        (for _array_element_2 (Variables|Default|GetPlayerRefArray)
          (if (!= _array_element_2 _array_element)
            (if (> (Math|Vector|Distance(Vector) (Transformation|GetActorLocation _array_element_2) (Transformation|GetActorLocation _array_element)) (LocalVariables|GetLongestDistBetweenPlayers))
              (LocalVariables|SetLongestDistBetweenPlayers (Math|Vector|Distance(Vector) (Transformation|GetActorLocation _array_element_2) (Transformation|GetActorLocation _array_element))))))
        (else
          (LocalVariables|SetAreAllPlayersValid false)
          (goto _label Break))))
    (:Completed
      (if (LocalVariables|GetAreAllPlayersValid)
        (Development|PrintString "Hello")
        (Transformation|SetWorldLocationAndRotation (Variables|Default|GetCameraPivot) (- (/ (LocalVariables|GetTotalPlayerLocationVectors) (Utilities|Array|Length (Variables|Default|GetPlayerRefArray))) "0,-75.000000,-50.000000") (Math|Rotator|FindLookatRotation (Transformation|GetWorldLocation (Variables|Default|GetCamera)) (/ (LocalVariables|GetTotalPlayerLocationVectors) (Utilities|Array|Length (Variables|Default|GetPlayerRefArray)))) false false)
        (Variables|/Script/Engine.SpringArmComponent|SetTargetArmLength (Variables|Default|GetSpringArm) (Math|Float|Clamp(Float) (+ (LocalVariables|GetLongestDistBetweenPlayers) 75.0) 5e+02 2.5e+03))
        (else
          (Development|PrintString "Invalid Player Ref"))))))
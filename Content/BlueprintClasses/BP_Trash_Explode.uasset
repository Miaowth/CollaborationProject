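; BP_Trash_Explode is a throwable trash object that explodes on impact once thrown.
; Its Hit event ignores the BP_Character whose PlayerID matches PlayerInt, but accepts other characters and non-character hits.
; A DoOnce gate then fires a radial force impulse, spawns an explosion particle at the hit location and destroys the actor after a brief delay.
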(event Collision|EventHit
  (params (MyComp :type Primitive%20Component%20Object%20Reference) (Other :type Actor%20Object%20Reference) (OtherComp :type Primitive%20Component%20Object%20Reference) (bSelfMoved :type Boolean) (HitLocation :type Vector :default "0, 0, 0") (HitNormal :type Vector :default "0, 0, 0") (NormalImpulse :type Vector :default "0, 0, 0") (Hit :type Hit%20Result%20Structure%20%28by%20ref%29))
  (bind _asbp_character (Utilities|Casting|CastToBP_Character (Components|GetOwner OtherComp))
    (:then
      (if (!= (Variables|Default|GetPlayerInt) (Variables|/Game/BlueprintClasses/BP_Character.BP_Character_C|GetPlayerID _asbp_character))
        (if (Variables|Default|GetThrown?) :!label _label
          (Utilities|FlowControl|DoOnce false
            (:Completed
              (Class|RadialForceComponent|FireImpulse (Variables|Default|GetRadialForce))
              (Effects|SpawnEmitteratLocation "/Game/Assets/FX/PS_Explode.PS_Explode" HitLocation)
              (Utilities|FlowControl|Delay 0.2)
              (Actor|DestroyActor))))))
    (:CastFailed
      (goto _label))))

(fn ConstructionScript
  (|CallParentFunction))
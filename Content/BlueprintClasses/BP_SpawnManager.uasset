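; BP_SpawnManager periodically spawns BP_TestTrash actors around its own location.
; On BeginPlay it starts a looping timer with a short, randomized initial delay.
; Each tick of the timer spawns trash at a random horizontal offset, always spawning with collision adjustment, then applies a random velocity-change impulse to its Sphere component.
; The spawn area and impulse ranges are hardcoded.
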(event Custom|SpawnTrash
  (bind _returnvalue (Transformation|GetActorTransform))
  ;[1 0.4624 0.7808] At the start of the game, create a timer to randomly spawn trash within an area and add some force to it. //TODO EXT - make float ranges designer accessible
  (bind _returnvalue_2 (Game|SpawnActorfromClass "/Game/BlueprintClasses/BP_TestTrash.BP_TestTrash_C" (Math|Transform|MakeTransform (Math|Vector|MakeVector (+ (.x (.location _returnvalue)) (Math|Random|RandomFloatinRange -1e+02 1e+02)) (+ (.y (.location _returnvalue)) (Math|Random|RandomFloatinRange -1e+02 1e+02)) (.z (.location _returnvalue))) (.rotation _returnvalue) (.scale _returnvalue)) "AdjustIfPossibleButAlwaysSpawn" 0 0))
  (Physics|AddImpulse (Variables|/Game/BlueprintClasses/BP_TestTrash.BP_TestTrash_C|GetSphere _returnvalue_2) (Math|Vector|MakeVector (Math|Random|RandomFloatinRange -5e+01 5e+01) (Math|Random|RandomFloatinRange -5e+01 5e+01) (Math|Random|RandomFloatinRange -5e+01 5e+01)) "None" true))

(event EventBeginPlay
  ;[1 0.4624 0.7808] At the start of the game, create a timer to randomly spawn trash within an area and add some force to it. //TODO EXT - make float ranges designer accessible
  (Utilities|Time|SetTimerbyEvent (delegate Custom|SpawnTrash) 3.0 true 1.0 1.0))

(fn ConstructionScript)
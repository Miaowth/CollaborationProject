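; Game mode for a timed, score-based local multiplayer level that announces a winner when time runs out.
; BeginPlay creates an additional local player, and Tick accumulates and prints elapsed time while the timer is active until it reaches the level time.
; FindWinningPlayer then compares points across all BP_PointArea actors, returning the leader's player number or -1 for a tie.
; Results and score comparisons are shown only through debug prints.
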(event EventBeginPlay
  (Class|GameplayStatics|CreatePlayer -1))

(event EventTick
  (params (DeltaSeconds :type Float%20%28single-precision%29))
  (if (Variables|Default|GetIsTimerActive)
    (bind _output_get (Variables|Default|SetTotalTime (+ DeltaSeconds (Variables|Default|GetTotalTime))))
    (if (<= (Variables|Default|GetLevelTime) _output_get)
      (Development|PrintString "Level Over!")
      (Variables|Default|SetIsTimerActive false)
      ;[1 0.4689 0.8391] checks if there is a winner or a tie
      (bind _winningplayernum (CallFunction|FindWinningPlayer))
      (if (!= _winningplayernum -1)
        (Development|PrintString (Utilities|String|BuildString(Integer) "The Winner is player" "" _winningplayernum "!"))
        (else
          (Development|PrintString "No Winner")))
      (else
        (Development|PrintString (Utilities|String|ToString(Float) _output_get))))))

(fn ConstructionScript)

(fn FindWinningPlayer
  (bind _outactors (Actor|GetAllActorsOfClass "/Game/BlueprintClasses/BP_PointArea.BP_PointArea_C"))
  (for (_array_element _array_index) _outactors
    (if (> (Variables|/Game/BlueprintClasses/BP_PointArea.BP_PointArea_C|GetPointsTotal _array_element) (LocalVariables|GetTopScore))
      (LocalVariables|SetTopScoreIndex _array_index)
      (LocalVariables|SetTopScore (Variables|/Game/BlueprintClasses/BP_PointArea.BP_PointArea_C|GetPointsTotal _array_element))
      (Development|PrintString "New High Score")
      (LocalVariables|SetTopPlayerNum (Variables|/Game/BlueprintClasses/BP_PointArea.BP_PointArea_C|GetPlayerNumber _array_element))
      (elif (== (Variables|/Game/BlueprintClasses/BP_PointArea.BP_PointArea_C|GetPointsTotal _array_element) (LocalVariables|GetTopScore))
        ;[1 0.4324 0.8792] sets top player back to -1 to indicate no current leader
        (Development|PrintString "TIE!")
        (LocalVariables|SetTopScoreIndex -1)
        (LocalVariables|SetTopPlayerNum -1)
        (else
          (Development|PrintString "High Score Remains")))))
  (return (LocalVariables|GetTopPlayerNum)))